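; Floor tile that changes color while a CharacterBase stands on it and falls once it turns red.
; Overlap events on FloorCollision set a touch flag that lets Tick drive ChangeColor at a configurable speed.
; ChangeColor lowers blue, then green, feeding a dynamic material created in the construction script.
; When both channels reach zero, FloorFall enables physics simulation on the floor mesh.
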(event `self.ReceiveBeginPlay`)

(event `self.ReceiveTick`
  (params (DeltaSeconds :type "Float (single-precision)"))
  (bind _color (`self.Color`))
  (bind (_r _g _b) (break `LinearColor` _color))
  (if (`self.IsTouchCharacter`)
    (`self.ChangeColor` (* DeltaSeconds (`self.SpeedOfColorChanging`)))
    (`MaterialInstanceDynamic.SetVectorParameterValue` (`self.DynamicMaterial`) "Color" _color)
    ;[1 1 1] Is Floor Red
    (if (== _b 0.0)
      (if (== _g 0.0)
        (`self.FloorFall`)))))

(event `self.FloorCollision.OnComponentBeginOverlap`
  (params (OverlappedComponent :type "PrimitiveComponent Object Reference") (OtherActor :type "Actor Object Reference") (OtherComp :type "PrimitiveComponent Object Reference") (OtherBodyIndex :type Integer) (bFromSweep :type Boolean) (SweepResult :type "HitResult Structure (by ref)"))
  (cast `/Game/ThirdPersonBP/Blueprints/CharacterBase` OtherActor)
  (set `self.IsTouchCharacter` true))

(event `self.FloorCollision.OnComponentEndOverlap`
  (params (OverlappedComponent :type "PrimitiveComponent Object Reference") (OtherActor :type "Actor Object Reference") (OtherComp :type "PrimitiveComponent Object Reference") (OtherBodyIndex :type Integer))
  (cast `/Game/ThirdPersonBP/Blueprints/CharacterBase` OtherActor)
  (set `self.IsTouchCharacter` false))

(fn `ChangeColor`
  (params (Delta :type "Float (double-precision)"))
  (locals (ResultG :type "Float (double-precision)" :default 1.0) (ResultB :type "Float (double-precision)" :default 1.0))
  (bind (_r _g _b _a) (`KismetMathLibrary.BreakColor` (`self.Color`)))
  (if (> _b 0.0)
    (set `local.ResultB` (`KismetMathLibrary.FClamp` (- _b Delta)))
    (bind _output_get (set `self.Color` (`KismetMathLibrary.MakeColor` _r (`local.ResultG`) (`local.ResultB`) _a) :!label _label))
    (elif (> _g 0.0)
      (set `local.ResultB` 0.0)
      (set `local.ResultG` (`KismetMathLibrary.FClamp` (- _g Delta)))
      (goto _label))))

(fn `FloorFall`
  (`PrimitiveComponent.SetSimulatePhysics` (`self.SM_Floor`) true))

(fn `UserConstructionScript`
  (bind _returnvalue (`PrimitiveComponent.CreateDynamicMaterialInstance` (`self.SM_Floor`) 0 null))
  (set `self.DynamicMaterial` _returnvalue))